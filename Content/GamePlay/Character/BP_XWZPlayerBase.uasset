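; Base player character Blueprint handling camera input, camera-relative movement, jumping and falling.
; Tick picks a facing yaw from input or the battle target, then sends it through server/client-style input events that smooth turning with a speed-based curve.
; Projectile-path prediction estimates fall time to scale the anim Blueprint's falling rate, and jumps briefly delay after setting an animation flag.
; Keys adjust animation rate and toggle synced root motion mode.
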(event `self.ReceiveTick`
  (params (DeltaSeconds :type "Float (single-precision)"))
  (bind (_returnvalue_x _returnvalue_y _returnvalue_z) (`KismetMathLibrary.BreakVector` (`self.GetVelocity`)))
  (bind (_returnvalue_roll _returnvalue_pitch _returnvalue_yaw) (`KismetMathLibrary.BreakRotator` (`self.GetControlRotation`)))
  (bind _returnvalue (`SkeletalMeshComponent.GetAnimInstance` (`self.Mesh`)))
  (bind (_returnvalue_roll_2 _returnvalue_pitch_2 _returnvalue_yaw_2) (`KismetMathLibrary.BreakRotator` (`SceneComponent.K2_GetComponentRotation` (`self.CapsuleComponent`))))
  (bind (_returnvalue_roll_3 _returnvalue_pitch_3 _returnvalue_yaw_3) (`KismetMathLibrary.BreakRotator` (`KismetMathLibrary.FindLookAtRotation` (`self.K2_GetActorLocation`) (`self.K2_GetActorLocation` (`self.CurrentTarget`)))))
  ;[1 1 1] TickAnd state
  (`parent.ReceiveTick` DeltaSeconds)
  ;;[1 1 1] 下落处理
  (set `self._deltaTime` DeltaSeconds)
  (if (`NavMovementComponent.IsFalling` (`self.CharacterMovement`))
    (if (and (< _returnvalue_z 0.0) (not (`self.AlreadyCheckFall`)))
      (bind _time (`self.CheckFallTime`))
      (bind _asplayer_base_animation_bp (cast `/Game/GamePlay/Animation/PlayerBaseAnimationBP` _returnvalue))
      (set `/Game/GamePlay/Animation/PlayerBaseAnimationBP.FallingRate` (/ 0.333 _time) _asplayer_base_animation_bp)
      (set `self.AlreadyCheckFall` true))
    (else
      (if (`self.AlreadyCheckFall`)
        (set `self.AlreadyCheckFall` false)
        (bind _asplayer_base_animation_bp_2 (cast `/Game/GamePlay/Animation/PlayerBaseAnimationBP` _returnvalue))
        (set `/Game/GamePlay/Animation/PlayerBaseAnimationBP.FallingRate` 0.0 _asplayer_base_animation_bp_2))
      (if (`|EnumEquality` (`CharacterMovementComponent.MovementMode` (`self.CharacterMovement`)) "MOVE_Walking")
        ;;[1 1 1] 更新TargetYaw
        (if (`self.bInBattle`)
          (if (`KismetSystemLibrary.IsValid` (`self.CurrentTarget`))
            (set `self.FaceYaw` _returnvalue_yaw_3)
            (if (`self.CanMove`) :!label _label
              (`self.AddMovementInput` (stale _output_get))
              (`self.S_Input` (stale _output_get) (stale _output_get_2)))
            (else
              (if (`self.IsLocallyControlled`) :!label _label_2
                (bind _output_get (set `self.worldInput` (`KismetMathLibrary.Normal` (`KismetMathLibrary.GreaterGreater_VectorRotator` (`KismetMathLibrary.MakeVector` (`self.GetInputAxisValue`) (`self.GetInputAxisValue`)) (`KismetMathLibrary.MakeRotator` 0.0 0.0 _returnvalue_yaw)))))
                (bind _output_get_2 (set `self.FaceYaw` (`KismetMathLibrary.SelectFloat` _returnvalue_yaw_2 (`self.GetInputDir` _output_get (`self.S_CurYaw`)) (`self.bInBattle`))))
                (goto _label))))
          (else
            (goto _label_2)))))))

(event `InputAxis|CameraPitch`
  (params (AxisValue :type "Float (single-precision)"))
  ;[1 1 1] TickAnd state
  (`self.AddControllerPitchInput` AxisValue))

(event `InputAxis|CameraYaw`
  (params (AxisValue :type "Float (single-precision)"))
  ;[1 1 1] TickAnd state
  (`self.AddControllerYawInput` AxisValue))

(event `InputAction|Action`
  (params (Key :type "Key Structure"))
  ;[1 1 1] TickAnd state
  (:`Pressed`
    (set `self.bInAction` true))
  (:`Released`
    (set `self.bInAction` false)))

(event `S_Input`
  (params (WorldInput :type "Vector Structure") (TargeYaw :type "Float (double-precision)"))
  (bind (_returnvalue_roll _returnvalue_pitch _returnvalue_yaw) (`KismetMathLibrary.BreakRotator` (`SceneComponent.K2_GetComponentRotation` (`self.CapsuleComponent`))))
  ;[1 1 1] TickAnd state
  ;;[1 1 1] 通用移动处理
  (bind _output_get (set `self.worldInput` WorldInput))
  (bind _output_get_2 (set `self.FaceYaw` (`KismetMathLibrary.SelectFloat` _returnvalue_yaw (`self.GetInputDir` _output_get (`self.S_CurYaw`)) (`self.bInBattle`))))
  (bind (_returnvalue_roll_2 _returnvalue_pitch_2 _returnvalue_yaw_2) (`KismetMathLibrary.BreakRotator` (`KismetMathLibrary.RInterpTo` (`KismetMathLibrary.MakeRotator` 0.0 0.0 (`self.S_CurYaw`)) (`KismetMathLibrary.MakeRotator` 0.0 0.0 _output_get_2) (`self._deltaTime`) (`CurveFloat.GetFloatValue` (`self.turnCurve`) (/ (`KismetMathLibrary.VSize` (`self.GetVelocity`)) (`MovementComponent.GetMaxSpeed` (`self.CharacterMovement`)))))))
  (`self.C_Input` _output_get _output_get_2 _returnvalue_yaw_2))

(event `S_ChangeRootMotionMode`
  (params (isRootMotionEnable :type Boolean))
  ;[1 1 1] TickAnd state
  ;;[1 1 1] 通用移动处理
  (bind _output_get (set `self.isRootMotion` isRootMotionEnable))
  (`AnimInstance.SetRootMotionMode` (`SkeletalMeshComponent.GetAnimInstance` (`self.Mesh`)) (select `bool` _output_get :`false` "RootMotionFromMontagesOnly" :`true` "RootMotionFromEverything" :!type "ERootMotionMode Enum")))

(event `C_ChangeRootMotionMode`
  (params (isRootMotionEnable :type Boolean))
  ;[1 1 1] TickAnd state
  ;;[1 1 1] 通用移动处理
  (bind _output_get (set `self.isRootMotion` isRootMotionEnable))
  (`AnimInstance.SetRootMotionMode` (`SkeletalMeshComponent.GetAnimInstance` (`self.Mesh`)) (select `bool` _output_get :`false` "RootMotionFromMontagesOnly" :`true` "RootMotionFromEverything" :!type "ERootMotionMode Enum")))

(event `Key|Add`
  (params (Key :type "Key Structure"))
  (bind _mesh (`self.Mesh`))
  ;[1 1 1] TickAnd state
  ;;[1 1 1] 通用移动处理
  (:`Pressed`
    (set `SkeletalMeshComponent.GlobalAnimRateScale` (`KismetMathLibrary.FClamp` (+ (`SkeletalMeshComponent.GlobalAnimRateScale` _mesh) 0.1) 0.1 2.0) _mesh)))

(event `/Game/Art/Blueprints/Interface/IAnimable.SetMeshRot`
  (params (NewRotYaw :type "Float (single-precision)"))
  ;[1 1 1] TickAnd state
  ;;[1 1 1] 通用移动处理
  (`SceneComponent.K2_SetWorldRotation` (`self.Mesh`) (`KismetMathLibrary.MakeRotator` 0.0 0.0 NewRotYaw) false false))

(event `C_Input`
  (params (WorldInput :type "Vector Structure") (TargetYaw :type "Float (double-precision)") (CurYaw :type "Float (double-precision)"))
  ;[1 1 1] TickAnd state
  ;;[1 1 1] 通用移动处理
  (if (not (`self.IsLocallyControlled`))
    (set `self.worldInput` WorldInput)
    (set `self.FaceYaw` TargetYaw))
  (set `self.S_CurYaw` CurYaw))

(event `Key|Subtract`
  (params (Key :type "Key Structure"))
  (bind _mesh (`self.Mesh`))
  ;[1 1 1] TickAnd state
  ;;[1 1 1] 通用移动处理
  (:`Pressed`
    (set `SkeletalMeshComponent.GlobalAnimRateScale` (`KismetMathLibrary.FClamp` (- (`SkeletalMeshComponent.GlobalAnimRateScale` _mesh) 0.1) 0.1 2.0) _mesh)))

(event `Key|Tab`
  (params (Key :type "Key Structure"))
  ;[1 1 1] TickAnd state
  ;;[1 1 1] 通用移动处理
  (:`Pressed`
    (bind _output_get (set `self.isRootMotion` (not (stale _output_get))))
    (`AnimInstance.SetRootMotionMode` (`SkeletalMeshComponent.GetAnimInstance` (`self.Mesh`)) (select `bool` _output_get :`false` "RootMotionFromMontagesOnly" :`true` "RootMotionFromEverything" :!type "ERootMotionMode Enum"))
    (`self.S_ChangeRootMotionMode` _output_get)))

(event `ExecuteJump`
  ;[1 1 1] TickAnd state
  ;;[1 1 1] 通用移动处理
  (bind _asplayer_base_animation_bp (cast `/Game/GamePlay/Animation/PlayerBaseAnimationBP` (`SkeletalMeshComponent.GetAnimInstance` (`self.Mesh`))))
  (set `/Game/GamePlay/Animation/PlayerBaseAnimationBP.JumpInAir` true _asplayer_base_animation_bp)
  (`KismetSystemLibrary.Delay` 0.15)
  (`self.Jump`)
  (set `/Game/GamePlay/Animation/PlayerBaseAnimationBP.JumpInAir` false _asplayer_base_animation_bp))

(fn `CheckFallTime`
  (returns (Time :type "Float (double-precision)"))
  (bind _predictresult (`GameplayStatics.Blueprint_PredictProjectilePath_Advanced` (make `PredictProjectilePathParams` (`self.K2_GetActorLocation`) (`self.GetVelocity`) true 5.0 5.0 false "ECC_Visibility" (`|MakeArray` "ObjectTypeQuery1" :!type "EObjectTypeQuery Enum") (`|MakeArray`))))
  (return (`.Time` (break `PredictProjectilePathPointData` (`.LastTraceDestination` (break `PredictProjectilePathResult` _predictresult))))))

(fn `GetBaseValue`
  (returns (Velocity :type "Vector Structure") (TargetYaw :type "Float (double-precision)") (ServerWordYaw :type "Float (double-precision)") (BaseAimRotation :type "Rotator Structure") (MovementMode :type "EMovementMode Enum"))
  (return (`self.GetVelocity`) (`self.FaceYaw`) (`self.S_CurYaw`) (`self.GetBaseAimRotation`) (`CharacterMovementComponent.MovementMode` (`self.CharacterMovement`))))

(fn `GetInputValue`
  (returns (WorldInput :type "Vector Structure") (isRootMotion :type Boolean))
  (return (`self.worldInput`) (`self.isRootMotion`)))

(fn `UserConstructionScript`
  (`parent.UserConstructionScript`))